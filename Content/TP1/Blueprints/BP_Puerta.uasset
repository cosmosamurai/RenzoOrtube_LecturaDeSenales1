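; BP_Puerta is a double door that opens once when an actor holding a key interacts with it.
; The Interactuar event checks the actor's TieneLlave, then sets Abierta and plays a Timeline, or prints a "find the key" message in Spanish when the key is missing.
; Each Timeline update adds its track values to the current X location of both leaves, so movement accumulates per tick rather than interpolating between fixed positions.
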(event EventBeginPlay)

(event Collision|EventActorBeginOverlap
  (params (OtherActor :type Actor%20Object%20Reference)))

(event EventTick
  (params (DeltaSeconds :type Float%20%28single-precision%29)))

(event EventInteractuar
  (params (Actor :type BP%20Third%20Person%20Character%20Object%20Reference))
  (bind _hojaderecha (Variables|Default|GetHojaDerecha))
  (bind _hojaizquierda (Variables|Default|GetHojaIzquierda))
  (bind _relativelocation (Variables|/Script/Engine.SceneComponent|GetRelativeLocation _hojaderecha))
  (bind _relativelocation_2 (Variables|/Script/Engine.SceneComponent|GetRelativeLocation _hojaizquierda))
  (if (Variables|/Game/ThirdPerson/Blueprints/BP_ThirdPersonCharacter.BP_ThirdPersonCharacter_C|GetbTieneLlave Actor)
    (if (not (Variables|Default|GetbAbierta))
      (Variables|Default|SetbAbierta true)
      (bind (_direction _izquierada _derecha) (Timeline|Timeline Play)
        (:Update
          (Transformation|SetRelativeLocation _hojaizquierda (Math|Vector|MakeVector (+ (.x _relativelocation_2) _izquierada) (.y _relativelocation_2) (.z _relativelocation_2)) false false)
          (Transformation|SetRelativeLocation _hojaderecha (Math|Vector|MakeVector (+ (.x _relativelocation) _derecha) (.y _relativelocation) (.z _relativelocation)) false false))))
    (else
      (Development|PrintString "Busca la llave"))))

(fn ConstructionScript)

(fn NewFunction0)

(fn NewFunction)